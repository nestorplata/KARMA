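; BP_Statue is an interactable statue that takes an item offering from the player and triggers the win.
; Interacting removes ItemToConsume from the player's InventorySystem, first swapping in the player's inventory entry of that type when IsConsumingAll is set.
; A successful removal reveals the Incense hidden at BeginPlay and calls Win on BP_FirstPersonCharacter.
; Looking at it toggles render depth; SetIncenseVisible, a partial-reveal function, is never called here.
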(event EventBeginPlay
  (Rendering|SetVisibility (Variables|Default|GetIncense) false true))

(event Collision|EventActorBeginOverlap
  (params (OtherActor :type Actor%20Object%20Reference)))

(event EventTick
  (params (DeltaSeconds :type Float%20%28single-precision%29)))

(event EventInteractwith
  (params (FirstPersonCharacther :type BP%20First%20Person%20Character%20Object%20Reference))
  (bind _inventorysystem (Variables|/Game/FirstPerson/Blueprints/BP_FirstPersonCharacter.BP_FirstPersonCharacter_C|GetInventorySystem FirstPersonCharacther))
  (if (Variables|Default|GetIsConsumingAll)
    (bind _output (Default|GetItemRef _inventorysystem (.itemtype (Variables|Default|GetItemToConsume))))
    (Variables|Default|SetItemToConsume _output))
  (bind _success (Default|RemoveItem _inventorysystem (Variables|Default|GetItemToConsume)))
  (if _success
    (CallFunction|SetAllMeshesVisibe)
    (CallFunction|Win)))

(event EventLookat
  (params (isLookingAt :type Boolean))
  (CallFunction|ToogleRenderDepth isLookingAt self))

(fn ConstructionScript)

(fn SetAllMeshesVisibe
  (Rendering|SetVisibility (Variables|Default|GetIncense) true true))

(fn SetIncenseVisible
  (params (Total%20to%20Reveal :type Integer))
  (LocalVariables|SetLoopRepetitions Total%20to%20Reveal)
  (bind (_array_element _array_index) (Utilities|Array|ForEachLoopwithBreak (Components|GetChildrenComponents (Variables|Default|GetStatue) false) :!label _label)
    (:LoopBody
      (if (Variables|/Script/Engine.SceneComponent|GetbVisible _array_element)
        (Math|Integer|IncrementInt (LocalVariables|GetLoopRepetitions))
        (else
          (Rendering|SetVisibility _array_element true false)
          (if (== _array_index (- (LocalVariables|GetLoopRepetitions) -1))
            (goto _label Break)))))))

(fn Win
  (bind _asbp_first_person_character (Utilities|Casting|CastToBP_FirstPersonCharacter (Game|GetPlayerCharacter 0)))
  (Default|Win _asbp_first_person_character))