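; Game instance that saves and restores the player's position and current level through a single BP_SaveGame slot.
; SaveGame writes the character's transform and level name to the slot and prints a confirmation.
; LoadGameFromMenu sets WasGameLoaded, reads the slot, opens the saved level and switches to game-only input.
; A separate LoadGame function applies the cached transform to the player character, with no caller in this file.
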(event Custom|LoadGameFromMenu
  (bind _returnvalue (Game|GetPlayerController 0))
  (Variables|Default|SetWasGameLoaded true)
  (bind _savelevel (CallFunction|SaveLoadedGame))
  (Game|OpenLevel(byName) (Utilities|String|StringToName _savelevel))
  (Variables|/Script/Engine.PlayerController|SetbShowMouseCursor _returnvalue false)
  (Input|SetInputModeGameOnly _returnvalue false))

(fn SaveGame
  (bind _returnvalue (SaveGame|CreateSaveGameObject "/Game/Saving/BP_SaveGame.BP_SaveGame_C"))
  (bind _output_get (Variables|Default|SetSaveRef _returnvalue))
  (Variables|/Game/Saving/BP_SaveGame.BP_SaveGame_C|SetTransform _output_get (Transformation|GetActorTransform (Variables|Default|GetPlayerCharacter)))
  (bind _returnvalue_2 (Game|GetCurrentLevelName true))
  (Variables|/Game/Saving/BP_SaveGame.BP_SaveGame_C|SetSaveLevel (Variables|Default|GetSaveRef) _returnvalue_2)
  (SaveGame|SaveGametoSlot (Variables|Default|GetSaveRef) (Variables|Default|GetSlotNameSave))
  (Development|PrintString "Level has been saved "))

(fn SaveLoadedGame
  (bind _returnvalue (SaveGame|LoadGamefromSlot (Variables|Default|GetSlotNameSave)))
  (bind _asbp_save_game (Utilities|Casting|CastToBP_SaveGame _returnvalue))
  (bind _output_get (Variables|Default|SetSaveRef _asbp_save_game))
  (return (Variables|/Game/Saving/BP_SaveGame.BP_SaveGame_C|GetSaveLevel _output_get)))

(fn LoadGame
  (Transformation|SetActorTransform (Variables|Default|GetPlayerCharacter) (Variables|/Game/Saving/BP_SaveGame.BP_SaveGame_C|GetTransform (Variables|Default|GetSaveRef)))
  (if true
    _))